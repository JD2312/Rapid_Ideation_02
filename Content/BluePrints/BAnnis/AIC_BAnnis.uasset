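; AI controller for BP_BAnnis that makes the pawn follow the player character while following is allowed.
; On possess it caches the pawn cast to BP_BAnnis.
; Each tick it reads the pawn's CanFollow flag, either setting IsWalking and issuing AIMoveTo toward player 0, or clearing IsWalking and stopping movement.
; The move request is reissued every frame by polling, with no Behavior Tree in this graph.
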(event EventTick
  (params (DeltaSeconds :type Float%20%28single-precision%29))
  (bind _returnvalue (Game|GetPlayerCharacter 0))
  (bind _as_bp_bannis (Variables|Default|GetAs%20BP%20BAnnis)
    (:then
      (if (== (Variables|/Game/BluePrints/BAnnis/BP_BAnnis.BP_BAnnis_C|GetCanFollow _as_bp_bannis) true)
        (Variables|/Game/BluePrints/BAnnis/BP_BAnnis.BP_BAnnis_C|SetIsWalking _as_bp_bannis true)
        (AI|AIMoveTo _as_bp_bannis (Transformation|GetActorLocation _returnvalue) _returnvalue 5.0 false)
        (else
          (Variables|/Game/BluePrints/BAnnis/BP_BAnnis.BP_BAnnis_C|SetIsWalking _as_bp_bannis false)
          (Variables|/Game/BluePrints/BAnnis/BP_BAnnis.BP_BAnnis_C|SetCanFollow _as_bp_bannis false)
          (AI|Navigation|StopMovement))))
    (:else)))

(event EventPossess
  (params (PossessedPawn :type Pawn%20Object%20Reference))
  (bind _asbp_bannis (Utilities|Casting|CastToBP_BAnnis PossessedPawn))
  (Variables|Default|SetAs%20BP%20BAnnis _asbp_bannis))

(fn ConstructionScript)