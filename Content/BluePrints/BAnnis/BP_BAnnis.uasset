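; BP_BAnnis is a sprite-based enemy character with a health bar widget that fights the player across two depth lanes.
; Tick faces the player's GameInstance location, counts a frame-based attack cooldown and slides between Y lanes when trigger boxes flag it.
; Overlap volumes set follow state and start random light or special attacks, though the special's ApplyDamage has no target.
; Damage launches it, pauses following and, at zero health, destroys it and decrements EnemiesInBattle.
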(event OnComponentBeginOverlap(Sight)
  (params (OverlappedComponent :type Primitive%20Component%20Object%20Reference) (OtherActor :type Actor%20Object%20Reference) (OtherComp :type Primitive%20Component%20Object%20Reference) (OtherBodyIndex :type Integer) (bFromSweep :type Boolean) (SweepResult :type Hit%20Result%20Structure%20%28by%20ref%29))
  (if (Utilities|DoesObjectImplementInterface OtherActor "/Game/BluePrints/Interfaces/BPI_Player.BPI_Player_C")
    (Variables|Default|SetCanFollow true)
    (Variables|Default|SetPlayerLocation (Transformation|GetActorLocation OtherActor))))

(event OnComponentEndOverlap(Sight)
  (params (OverlappedComponent :type Primitive%20Component%20Object%20Reference) (OtherActor :type Actor%20Object%20Reference) (OtherComp :type Primitive%20Component%20Object%20Reference) (OtherBodyIndex :type Integer))
  (if (Utilities|DoesObjectImplementInterface OtherActor "/Game/BluePrints/Interfaces/BPI_Player.BPI_Player_C")
    (Variables|Default|SetCanFollow false)
    (Variables|Default|SetIsWalking false)))

(event OnComponentBeginOverlap(AttackRange)
  (params (OverlappedComponent :type Primitive%20Component%20Object%20Reference) (OtherActor :type Actor%20Object%20Reference) (OtherComp :type Primitive%20Component%20Object%20Reference) (OtherBodyIndex :type Integer) (bFromSweep :type Boolean) (SweepResult :type Hit%20Result%20Structure%20%28by%20ref%29))
  (if (Utilities|DoesObjectImplementInterface OtherActor "/Game/BluePrints/Interfaces/BPI_Player.BPI_Player_C")
    (if (== (Variables|Default|GetCanAttack) true)
      (if (Math|Integer|InRange(Integer) (Math|Random|RandomIntegerinRange 0 10) 4 10)
        (Variables|Default|SetIsLightAtt true)
        (Utilities|FlowControl|Delay 1.0)
        (Game|Damage|ApplyDamage OtherActor 1e+01 0 0)
        (Utilities|FlowControl|Delay 1.0)
        (Variables|Default|SetIsLightAtt false)
        (Variables|Default|SetIsSpecialAtt false)
        (Variables|Default|SetCanAttack false)
        (else
          (Variables|Default|SetIsSpecialAtt true)
          (Utilities|FlowControl|Delay 1.0)
          (Game|Damage|ApplyDamage 0 2e+01 0 0)
          (Utilities|FlowControl|Delay 2.0)
          (Variables|Default|SetIsLightAtt false)
          (Variables|Default|SetIsSpecialAtt false)
          (Variables|Default|SetCanAttack false))))))

(event OnComponentBeginOverlap(Box_MoveFore)
  (params (OverlappedComponent :type Primitive%20Component%20Object%20Reference) (OtherActor :type Actor%20Object%20Reference) (OtherComp :type Primitive%20Component%20Object%20Reference) (OtherBodyIndex :type Integer) (bFromSweep :type Boolean) (SweepResult :type Hit%20Result%20Structure%20%28by%20ref%29))
  (if (Utilities|DoesObjectImplementInterface OtherActor "/Game/BluePrints/Interfaces/BPI_Player.BPI_Player_C")
    (Variables|Default|SetMoveForewards true)))

(event OnComponentBeginOverlap(Box_MoveBack)
  (params (OverlappedComponent :type Primitive%20Component%20Object%20Reference) (OtherActor :type Actor%20Object%20Reference) (OtherComp :type Primitive%20Component%20Object%20Reference) (OtherBodyIndex :type Integer) (bFromSweep :type Boolean) (SweepResult :type Hit%20Result%20Structure%20%28by%20ref%29))
  (if (Utilities|DoesObjectImplementInterface OtherActor "/Game/BluePrints/Interfaces/BPI_Player.BPI_Player_C")
    (Variables|Default|SetMoveBackwards true)))

(event Custom|MoveForward
  (Pawn|Input|AddMovementInput (Transformation|GetActorForwardVector) 1.0 false)
  (Variables|Default|SetIsWalking true))

(event Custom|UpdateRotation
  (bind _sprite (Variables|Default|GetSprite))
  (Math|Float|CompareFloat (.x (Variables|/Script/Engine.MovementComponent|GetVelocity (Variables|Character|GetCharacterMovement))) 0.0
    (:>
      (Transformation|SetRelativeRotation _sprite "0, 0, 0" false false))
    (:<
      (Transformation|SetRelativeRotation _sprite "0.000000,-180.000000,0.000000" false false))))

(event EventBeginPlay
  (CallFunction|UpdateHealthBar)
  (bind _asgi_game_instance (Utilities|Casting|CastToGI_GameInstance (Game|GetGameInstance)))
  (bind _output_get (Variables|Default|SetAs%20GI%20Game%20Instance _asgi_game_instance))
  (Variables|Default|SetWherePlayer (Variables|/Game/BluePrints/GI_GameInstance.GI_GameInstance_C|GetWherePlayer _output_get))
  (Variables|Default|SetWhereSelf 1))

(event Collision|EventActorBeginOverlap
  (params (OtherActor :type Actor%20Object%20Reference)))

(event EventTick
  (params (DeltaSeconds :type Float%20%28single-precision%29))
  (bind _capsulecomponent (Variables|Default|GetCapsuleComponent))
  (bind _capsulecomponent_2 (Variables|Default|GetCapsuleComponent))
  (bind _capsulecomponent_3 (Variables|Default|GetCapsuleComponent))
  (bind _capsulecomponent_4 (Variables|Default|GetCapsuleComponent))
  (bind _returnvalue (Transformation|GetWorldLocation _capsulecomponent_4))
  (bind _returnvalue_2 (Transformation|GetWorldLocation _capsulecomponent))
  (bind _returnvalue_3 (Transformation|GetWorldLocation _capsulecomponent_3))
  (bind _returnvalue_4 (Transformation|GetWorldLocation _capsulecomponent_2))
  (bind _returnvalue_5 (Math|Interpolation|VInterptoConstant (Math|Vector|MakeVector (.x _returnvalue) (.y _returnvalue) (.z _returnvalue)) (Math|Vector|MakeVector (.x _returnvalue) -2e+02 (.z _returnvalue)) DeltaSeconds 4.5e+02))
  (bind _returnvalue_6 (Math|Interpolation|VInterptoConstant (Math|Vector|MakeVector (.x _returnvalue_2) (.y _returnvalue_2) (.z _returnvalue_2)) (Math|Vector|MakeVector (.x _returnvalue_2) 0.0 (.z _returnvalue_2)) DeltaSeconds 4.5e+02))
  (if (> (.x (Variables|/Game/BluePrints/GI_GameInstance.GI_GameInstance_C|GetPlayerLocation (Variables|Default|GetAs%20GI%20Game%20Instance))) (.x (Transformation|GetWorldLocation (Variables|Default|GetCapsuleComponent))))
    (Transformation|SetActorRotation "0, 0, 0")
    (else
      (Transformation|SetActorRotation "0.000000,-180.000000,0.000000")))
  (if (== (Variables|Default|GetCanAttack) false)
    (Variables|Default|SetAttackCooldown (+ (Variables|Default|GetAttackCooldown) 1))
    (if (== (Variables|Default|GetAttackCooldown) 300)
      (Variables|Default|SetCanAttack true)
      (Variables|Default|SetAttackCooldown 0)
      (else
        (if (== (Variables|Default|GetMoveBackwards) true) :!label _label
          (Transformation|SetWorldLocation _capsulecomponent_4 (Math|Vector|MakeVector (.x _returnvalue_5) (.y _returnvalue_5) (.z _returnvalue_5)) false false)
          (if (Utilities|Operators|EqualEqual (Math|Vector|MakeVector (.x _returnvalue_4) (.y _returnvalue_4) (.z _returnvalue_4)) (Math|Vector|MakeVector (.x _returnvalue_4) -2e+02 (.z _returnvalue_4)) 0.0)
            (Variables|Default|SetMoveBackwards false)
            (Variables|Default|SetWhereSelf 2))
          (elif (== (Variables|Default|GetMoveForewards) true)
            (Transformation|SetWorldLocation _capsulecomponent (Math|Vector|MakeVector (.x _returnvalue_6) (.y _returnvalue_6) (.z _returnvalue_6)) false false)
            (if (Utilities|Operators|EqualEqual (Math|Vector|MakeVector (.x _returnvalue_3) (.y _returnvalue_3) (.z _returnvalue_3)) (Math|Vector|MakeVector (.x _returnvalue_3) 0.0 (.z _returnvalue_3)) 0.0)
              (Variables|Default|SetMoveForewards false)
              (Variables|Default|SetWhereSelf 1))))))
    (else
      (goto _label))))

(event Game|Damage|EventAnyDamage
  (params (Damage :type Float%20%28single-precision%29) (DamageType :type Damage%20Type%20Object%20Reference) (InstigatedBy :type Controller%20Object%20Reference) (DamageCauser :type Actor%20Object%20Reference))
  (Variables|Default|SetHealth (- (Variables|Default|GetHealth) Damage))
  (Character|LaunchCharacter "2500.000000,0.000000,0.000000" false false)
  (Variables|Default|SetIsDamaged true)
  (Variables|Default|SetCanFollow false)
  (CallFunction|UpdateHealthBar)
  (Utilities|FlowControl|Delay 1.0)
  (Variables|Default|SetCanFollow true)
  (Variables|Default|SetIsDamaged false)
  (if (<= (Variables|Default|GetHealth) 0.0)
    (Actor|DestroyActor)
    (bind _asgi_game_instance (Utilities|Casting|CastToGI_GameInstance (Game|GetGameInstance)))
    (Variables|/Game/BluePrints/GI_GameInstance.GI_GameInstance_C|SetEnemiesInBattle _asgi_game_instance (- (Variables|/Game/BluePrints/GI_GameInstance.GI_GameInstance_C|GetEnemiesInBattle _asgi_game_instance) 1))))

(fn ConstructionScript)

(fn UpdateHealthBar
  (bind _aswid_health (Utilities|Casting|CastToWID_Health (UserInterface|GetUserWidgetObject (Variables|Default|GetHealthWid))))
  (Variables|/Game/BluePrints/Widgets/WID_Health.WID_Health_C|SetHealth _aswid_health (Variables|Default|GetHealth))
  (return))