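; AN_Attack01 is an animation notify, apparently PaperZD, that deals melee hit damage for the main character's first attack.
; When fired with a valid owning instance, it runs a box overlap for pawns centered on the sequence render component, ignoring the owning actor.
; Each overlapped actor takes a small fixed damage and has its name printed for debugging.
; An "Empty" debug message prints after the loop, even when targets were hit.
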(fn OnReceiveNotify
  (params (OwningInstance :type Paper%20ZD%20Anim%20Instance%20Object%20Reference))
  (Utilities|IsValid OwningInstance
    (:Is%20Valid
      (bind _outactors (Collision|BoxOverlapActors (Transformation|GetWorldLocation (Variables|Default|GetSequenceRenderComponent)) "50.000000,50.000000,50.000000" (Utilities|Array|MakeArray "ObjectTypeQuery3") 0 (Utilities|Array|MakeArray (Class|PaperZDAnimInstance|GetOwningActor OwningInstance)) :!class /Script/Engine.KismetSystemLibrary))
      (for _array_element _outactors
        (Development|PrintString (Utilities|GetDisplayName _array_element))
        (Game|Damage|ApplyDamage _array_element 2.5 0 0))
      (Development|PrintString "Empty"))))